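; SetToPoints is a custom PCG Blueprint element that sets Density on a random subset of points in each spatial input.
; It converts each input to point data, then shuffles point indices and takes the leading entries, with WindowPoints setting the selection size.
; A collapsed graph rewrites the matching points and outputs the full point set with original tags and pin.
; The index arrays and any WindowPoints adjustment carry over between inputs without a reset.
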(fn ExecutewithContext
  (params (InContext :type PCG%20Context%20Structure%20%28by%20ref%29) (Input :type PCG%20Data%20Collection%20Structure%20%28by%20ref%29))
  (bind _returnvalue (Class|PCGDataFunctionLibrary|GetInputs Input))
  (for _array_element _returnvalue
    (LocalVariables|SetTags (.Tags (Utilities|Struct|BreakPCGTaggedData _array_element)))
    (LocalVariables|SetPins (.Pin (Utilities|Struct|BreakPCGTaggedData _array_element)))
    (bind _aspcgspatial_data (Utilities|Casting|CastToPCGSpatialData (.Data (Utilities|Struct|BreakPCGTaggedData _array_element))))
    (bind _output_get (LocalVariables|SetPCGPointData (SpatialData|ToPointDatawithContext _aspcgspatial_data (LocalVariables|GetContext))))
    (bind _output_get_2 (LocalVariables|SetPCGPoints (SpatialData|GetPoints _output_get)))
    (LocalVariables|SetPointCount (Utilities|Array|Length _output_get_2))
    (LocalVariables|SetSelectedMaxPoints (> (Variables|Default|GetWindowPoints) (LocalVariables|GetPointCount)))
    (for _index (range 0 (LocalVariables|GetPointCount))
      (Utilities|Array|Add (LocalVariables|GetIndexTracker) _index))
    (Utilities|Array|Shuffle (LocalVariables|GetIndexTracker))
    (if (LocalVariables|GetSelectedMaxPoints)
      (Variables|Default|SetWindowPoints (+ (LocalVariables|GetPointCount) 1)))
    (for _index_2 (range 0 (Variables|Default|GetWindowPoints))
      (Utilities|Array|Add (LocalVariables|GetIndexesToSelect) (Utilities|Array|Get(acopy) (LocalVariables|GetIndexTracker) _index_2)))
    (|PCGPointDataCollection))
  (return (Utilities|Struct|MakePCGDataCollection (LocalVariables|GetOutTaggedData))))