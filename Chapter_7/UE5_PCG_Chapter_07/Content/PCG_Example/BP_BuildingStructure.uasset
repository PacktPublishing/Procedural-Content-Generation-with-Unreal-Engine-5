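; Building actor that feeds its dimensions into a PCG graph instance, which by its parameter names lays out walls and floors.
; The construction script uses an Offsetter helper on DimensionOffset to set positive or reversed offsets for four walls and a pivot fix.
; It also sets height from DimensionOffset times NoOfFloors, a wall offset, and the negated actor location as CopyTransform.
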(event EventBeginPlay)

(event Collision|EventActorBeginOverlap
  (params (OtherActor :type Actor%20Object%20Reference)))

(event EventTick
  (params (DeltaSeconds :type Float%20%28single-precision%29)))

(fn ConstructionScript
  (bind _pcg (Variables|Default|GetPCG))
  (bind _dimensionoffset (Variables|Default|GetDimensionOffset))
  (bind (_offsetposition _reversedirection) (Utilities|Offsetter _dimensionoffset))
  (bind _graphinstance (Variables|/Script/PCG.PCGComponent|GetGraphInstance _pcg))
  (Utilities|FlowControl|Sequence
    (:then_0
      (Effects|Components|ParticleSystem|SetVectorParameter _graphinstance "Wall_West" (Math|Vector|MakeVector _offsetposition 0.0 0.0))
      (Effects|Components|ParticleSystem|SetVectorParameter _graphinstance "Wall_East" (Math|Vector|MakeVector _reversedirection 0.0 0.0))
      (Effects|Components|ParticleSystem|SetVectorParameter _graphinstance "Wall_North" (Math|Vector|MakeVector 0.0 _offsetposition 0.0))
      (Effects|Components|ParticleSystem|SetVectorParameter _graphinstance "Wall_South" (Math|Vector|MakeVector 0.0 _reversedirection 0.0))
      (Effects|Components|ParticleSystem|SetVectorParameter _graphinstance "FixingThePivot" (Math|Vector|MakeVector (.ReverseDirection (Utilities|Offsetter (Variables|Default|GetDimensionOffset))) 0.0 0.0)))
    (:then_1
      (Effects|Components|ParticleSystem|SetVectorParameter _graphinstance "Height" (Math|Vector|MakeVector 0.0 0.0 (* (Variables|Default|GetDimensionOffset) (Variables|Default|GetNoOfFloors))))
      (Effects|Components|ParticleSystem|SetVectorParameter _graphinstance "CopyTransform" (* (Transformation|GetActorLocation) -1.0))
      (Effects|Components|ParticleSystem|SetVectorParameter _graphinstance "WallsOffset" (Math|Vector|MakeVector (.OffsetPosition (Utilities|Offsetter (Variables|Default|GetWallsOffset))) 0.0 0.0)))))