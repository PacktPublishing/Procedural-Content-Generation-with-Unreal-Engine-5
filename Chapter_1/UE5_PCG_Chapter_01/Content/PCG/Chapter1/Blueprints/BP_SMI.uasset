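; BP_SMI is an actor Blueprint that lays out a flat grid of SM_Rock meshes through an Instanced Static Mesh component.
; The Construction Script assigns the mesh, then runs nested loops over the column and row spawn counts.
; Each pass adds an unrotated, unit-scale instance in local space, with X and Y set by loop index times a spacing variable.
; The event graph holds no active logic.
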(fn `UserConstructionScript`
  (`|ExecutionSequence`
    (:`then_0`
      ;[1 1 1] Instanced Meshes
      (`StaticMeshComponent.SetStaticMesh` (`self.InstancedStaticMesh`) "/Game/StarterContent/Props/SM_Rock.SM_Rock"))
    (:`then_1`
      ;[1 1 1] Grid Algorithm
      (for _index (range (+ (`self.SpawnPerColumn`) 1))
        (set `self.NumberOfInstances` (* (`self.InstancesPerRow`) _index))
        (for _index_2 (range (+ (`self.SpawnPerRow`) 1))
          ;[1 1 1] Adding instances
          (`InstancedStaticMeshComponent.AddInstance` (`self.InstancedStaticMesh`) (`KismetMathLibrary.MakeTransform` (`KismetMathLibrary.MakeVector` (`self.NumberOfInstances`) (* _index_2 (`self.InstancesPerColumn`)))) false))))))